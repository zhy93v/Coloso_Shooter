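; PSCharacter is a shooter player character Blueprint that handles movement, look and firing through Enhanced Input actions.
; Move actions add movement along the actor's forward and right vectors, while yaw and pitch actions feed controller rotation.
; The fire action casts the Child Actor component's actor to BP_PSGun and calls its Fire, leaving weapon logic to the gun.
; Overlap events and the construction script are empty.
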(event Input|EnhancedActionEvents|EnhancedInputActionPS_MoveForward
  (params (ActionValue :type Float%20%28double-precision%29) (ElapsedSeconds :type Float%20%28double-precision%29) (TriggeredSeconds :type Float%20%28double-precision%29) (InputAction :type Input%20Action%20Object%20Reference :default "/Game/ShooterContents/Input/PS_MoveForward.PS_MoveForward"))
  (:Triggered
    (Pawn|Input|AddMovementInput (Math|Vector|GetForwardVector (Transformation|GetActorRotation)) ActionValue false)))

(event Input|EnhancedActionEvents|EnhancedInputActionPS_MoveRight
  (params (ActionValue :type Float%20%28double-precision%29) (ElapsedSeconds :type Float%20%28double-precision%29) (TriggeredSeconds :type Float%20%28double-precision%29) (InputAction :type Input%20Action%20Object%20Reference :default "/Game/ShooterContents/Input/PS_MoveRight.PS_MoveRight"))
  (:Triggered
    (Pawn|Input|AddMovementInput (Math|Vector|GetRightVector (Transformation|GetActorRotation)) ActionValue false)))

(event Input|EnhancedActionEvents|EnhancedInputActionPS_MoveYaw
  (params (ActionValue :type Float%20%28double-precision%29) (ElapsedSeconds :type Float%20%28double-precision%29) (TriggeredSeconds :type Float%20%28double-precision%29) (InputAction :type Input%20Action%20Object%20Reference :default "/Game/ShooterContents/Input/PS_MoveYaw.PS_MoveYaw"))
  (:Triggered
    (Pawn|Input|AddControllerYawInput ActionValue)))

(event Input|EnhancedActionEvents|EnhancedInputActionPS_MovePitch
  (params (ActionValue :type Float%20%28double-precision%29) (ElapsedSeconds :type Float%20%28double-precision%29) (TriggeredSeconds :type Float%20%28double-precision%29) (InputAction :type Input%20Action%20Object%20Reference :default "/Game/ShooterContents/Input/PS_MovePitch.PS_MovePitch"))
  (:Triggered
    (Pawn|Input|AddControllerPitchInput ActionValue)))

(event Input|EnhancedActionEvents|EnhancedInputActionPS_Fire
  (params (ActionValue :type Boolean) (ElapsedSeconds :type Float%20%28double-precision%29) (TriggeredSeconds :type Float%20%28double-precision%29) (InputAction :type Input%20Action%20Object%20Reference :default "/Game/ShooterContents/Input/PS_Fire.PS_Fire"))
  (:Triggered
    (bind _asbp_psgun (Utilities|Casting|CastToBP_PSGun (Variables|/Script/Engine.ChildActorComponent|GetChildActor (Variables|Default|GetChildActor))))
    (Default|Fire _asbp_psgun)))

(event Collision|EventActorBeginOverlap
  (params (OtherActor :type Actor%20Object%20Reference)))

(event Collision|EventActorEndOverlap
  (params (OtherActor :type Actor%20Object%20Reference)))

(fn ConstructionScript)