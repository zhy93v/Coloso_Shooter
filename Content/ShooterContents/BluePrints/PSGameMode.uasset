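; Game mode for a shooter that tracks the match state, elapsed time and score.
; StartGame and EndGame advance the state from Ready to Playing to End, each acting only from the expected state, printing the new one and recording a timestamp.
; EndGame derives elapsed seconds from timespans built from day-to-millisecond clock fields, then passes any time left under a two-minute limit to AddScore as bonus points.
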(event EventBeginPlay)

(event EventTick
  (params (DeltaSeconds :type Float%20%28single-precision%29)))

(fn ConstructionScript)

(fn StartGame
  (switch Utilities|FlowControl|Switch|SwitchonStateOfGame (Variables|Default|GetState)
    (:NewEnumerator0
      (bind _output_get (Variables|Default|SetState "NewEnumerator1"))
      (Development|PrintString (Utilities|String|EnumtoString _output_get))
      (Variables|Default|SetStartTime (Math|DateTime|Now)))))

(fn EndGame
  (bind _starttime (Variables|Default|GetStartTime))
  (bind (_year _month _day _hour _minute _second _millisecond) (Math|DateTime|BreakDateTime _starttime))
  (switch Utilities|FlowControl|Switch|SwitchonStateOfGame (Variables|Default|GetState)
    (:NewEnumerator1
      (bind _output_get (Variables|Default|SetState "NewEnumerator2"))
      (Development|PrintString (Utilities|String|EnumtoString _output_get))
      (Variables|Default|SetEndTime (Math|DateTime|Now))
      (bind _output_get_2 (Variables|Default|SetEleapsedTime (/ (- (Class|KismetMathLibrary|GetTotalMilliseconds (Math|Timespan|MakeTimespan (.Day (Math|DateTime|BreakDateTime (Variables|Default|GetEndTime))) (.Hour (Math|DateTime|BreakDateTime (Variables|Default|GetEndTime))) (.Minute (Math|DateTime|BreakDateTime (Variables|Default|GetEndTime))) (.Second (Math|DateTime|BreakDateTime (Variables|Default|GetEndTime))) (.Millisecond (Math|DateTime|BreakDateTime (Variables|Default|GetEndTime))))) (Class|KismetMathLibrary|GetTotalMilliseconds (Math|Timespan|MakeTimespan _day _hour _minute _second _millisecond))) 1e+03)))
      (bind _output_get_3 (LocalVariables|SetTimeBonus (- 1.2e+02 _output_get_2)))
      (if (> _output_get_3 0.0)
        (CallFunction|AddScore (LocalVariables|GetTimeBonus))))))

(fn AddScore
  (params (NewParam :type Float%20%28double-precision%29))
  (Variables|Default|SetScore (+ NewParam (Variables|Default|GetScore))))