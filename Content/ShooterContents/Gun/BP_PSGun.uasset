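; BP_PSGun is a shooter gun that fires BP_PSBullet projectiles from a limited bullet count, with switchable semi-auto and full-auto modes.
; Fire spends a bullet, spawns the projectile at BulletSpawnPoint and sets its speed.
; In full auto, Fire re-arms a timer on itself after each shot until FireReleased clears it or bullets run out.
; Reload restores the maximum count, ChangeFireMode toggles modes, and GetUseType exposes the gun's use type.
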(event EventBeginPlay)

(event Collision|EventActorBeginOverlap
  (params (OtherActor :type Actor%20Object%20Reference)))

(event EventTick
  (params (DeltaSeconds :type Float%20%28single-precision%29)))

(fn ConstructionScript)

(fn Fire
  (if (> (Variables|Default|GetRemainingBullets) 0)
    (Variables|Default|SetRemainingBullets (- (Variables|Default|GetRemainingBullets) 1))
    (Development|PrintString (Utilities|String|Append "PSGun / Fire / RemainingBullets = " (Utilities|String|ToString(Integer) (Variables|Default|GetRemainingBullets))))
    (bind _returnvalue (Game|SpawnActorfromClass "/Game/ShooterContents/Gun/BP_PSBullet.BP_PSBullet_C" (Transformation|GetWorldTransform (Variables|Default|GetBulletSpawnPoint)) "Undefined" 0 0))
    (Default|SetSpeed _returnvalue 1e+04)
    (switch Utilities|FlowControl|Switch|SwitchonFireMode (Variables|Default|GetFireMode)
      (:NewEnumerator1
        (bind _returnvalue_2 (Utilities|Time|SetTimerbyFunctionName 0 "Fire" (Variables|Default|GetDurationPerFire)))
        (Variables|Default|SetTimerFire _returnvalue_2)))))

(fn Reload
  (Variables|Default|SetRemainingBullets (Variables|Default|GetMaxRemainingBullets)))

(fn GetUseType
  (return (Variables|Default|GetUseType)))

(fn ChangeFireMode
  (switch Utilities|FlowControl|Switch|SwitchonFireMode (Variables|Default|GetFireMode)
    (:NewEnumerator0
      (Variables|Default|SetFireMode "NewEnumerator1"))
    (:NewEnumerator1
      (Variables|Default|SetFireMode "NewEnumerator0"))))

(fn FirePressed
  (CallFunction|Fire))

(fn FireReleased
  (Utilities|Time|ClearandInvalidateTimerbyHandle (Variables|Default|GetTimerFire)))