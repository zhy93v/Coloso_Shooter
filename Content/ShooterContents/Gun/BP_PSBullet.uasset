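; BP_PSBullet is a projectile bullet actor in the shooter's gun content that flies straight and destroys itself on impact.
; Each Tick it moves with a swept SetActorLocation along the Bullet component's forward vector, scaled by Speed and delta time rather than using a movement component.
; Speed is set through SetSpeed, and BeginPlay shrinks the Bullet component.
; On component hit it prints the struck actor's name and destroys itself.
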(event OnComponentHit(Bullet)
  (params (HitComponent :type Primitive%20Component%20Object%20Reference) (OtherActor :type Actor%20Object%20Reference) (OtherComp :type Primitive%20Component%20Object%20Reference) (NormalImpulse :type Vector :default "0, 0, 0") (Hit :type Hit%20Result%20Structure%20%28by%20ref%29))
  (Development|PrintString (Utilities|GetDisplayName OtherActor))
  (Actor|DestroyActor))

(event EventBeginPlay
  (Transformation|SetWorldScale3D (Variables|Default|GetBullet) "0.100000,0.100000,0.100000"))

(event Collision|EventActorBeginOverlap
  (params (OtherActor :type Actor%20Object%20Reference)))

(event EventTick
  (params (DeltaSeconds :type Float%20%28single-precision%29))
  (bind _bulletvector (CallFunction|CalculateMoveVector DeltaSeconds))
  (Transformation|SetActorLocation (+ _bulletvector (Transformation|GetActorLocation)) true false))

(fn ConstructionScript)

(fn CalculateMoveVector
  (params (DeltaTIme :type Float%20%28double-precision%29))
  (bind _bullet (Variables|Default|GetBullet))
  (bind _returnvalue (Math|Vector|GetForwardVector _bullet))
  (Variables|Default|SetDeltaSpeed (* DeltaTIme (Variables|Default|GetSpeed)))
  (return (Math|Vector|MakeVector (* (.x _returnvalue) (Variables|Default|GetDeltaSpeed)) (* (.y _returnvalue) (Variables|Default|GetDeltaSpeed)) (* (.z _returnvalue) (Variables|Default|GetDeltaSpeed)))))

(fn SetSpeed
  (params (Value :type Float%20%28double-precision%29))
  (Variables|Default|SetSpeed Value))