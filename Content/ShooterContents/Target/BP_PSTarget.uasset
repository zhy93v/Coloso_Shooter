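; BP_PSTarget is a shooting target that tips up when a PSCharacter triggers its stand-up volume and falls when hit by a BP_PSBullet.
; A knock-down volume also drops it, and a reset volume re-arms a knocked-down target to Ready.
; StandUp and KnockDown gate on TargetState and set a timed 90-degree pitch rotation.
; Tick applies that rotation incrementally, then advances the state to Standing or KnockedDown.
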(event OnComponentHit(TargetBoard)
  (params (HitComponent :type Primitive%20Component%20Object%20Reference) (OtherActor :type Actor%20Object%20Reference) (OtherComp :type Primitive%20Component%20Object%20Reference) (NormalImpulse :type Vector :default "0, 0, 0") (Hit :type Hit%20Result%20Structure%20%28by%20ref%29))
  (Utilities|Casting|CastToBP_PSBullet OtherActor)
  (CallFunction|KnockDown))

(event OnActorBeginOverlap(StandUpVolume)
  (params (OverlappedActor :type Actor%20Object%20Reference) (OtherActor :type Actor%20Object%20Reference))
  (Utilities|Casting|CastToPSCharacter OtherActor)
  (CallFunction|StandUp))

(event OnActorBeginOverlap(KnockDownVolume)
  (params (OverlappedActor :type Actor%20Object%20Reference) (OtherActor :type Actor%20Object%20Reference))
  (Utilities|Casting|CastToPSCharacter OtherActor)
  (CallFunction|KnockDown))

(event OnActorBeginOverlap(ResetVolume)
  (params (OverlappedActor :type Actor%20Object%20Reference) (OtherActor :type Actor%20Object%20Reference))
  (Utilities|Casting|CastToPSCharacter OtherActor)
  (if (Utilities|Enum|Equal(Enum) (Variables|Components|GetTargetState) "NewEnumerator2")
    (Variables|Components|SetTargetState "NewEnumerator0")))

(event EventBeginPlay)

(event Collision|EventActorBeginOverlap
  (params (OtherActor :type Actor%20Object%20Reference)))

(event EventTick
  (params (DeltaSeconds :type Float%20%28single-precision%29))
  (CallFunction|TickRotate DeltaSeconds))

(fn ConstructionScript)

(fn KnockDown
  (if (Utilities|Enum|Equal(Enum) (Variables|Components|GetTargetState) "NewEnumerator1")
    (Utilities|FlowControl|Sequence
      (:then_0
        (bind _output_get (Variables|Rotation|SetRotationTime (Variables|Rotation|GetRotationTimeDown)))
        (Variables|Rotation|SetRotationRemainTime _output_get))
      (:then_1
        (Variables|Rotation|SetRotationDegree 9e+01))
      (:then_2
        (Variables|Components|SetTargetState "NewEnumerator4")))))

(fn StandUp
  (if (Utilities|Enum|Equal(Enum) (Variables|Components|GetTargetState) "NewEnumerator0")
    (Utilities|FlowControl|Sequence
      (:then_0
        (bind _output_get (Variables|Rotation|SetRotationTime (Variables|Rotation|GetRotationTimeStandUp)))
        (Variables|Rotation|SetRotationRemainTime _output_get))
      (:then_1
        (Variables|Rotation|SetRotationDegree -9e+01))
      (:then_2
        (Variables|Components|SetTargetState "NewEnumerator3")))))

(fn TickRotate
  (params (DeltaTime :type Float%20%28double-precision%29))
  (if (>= (Variables|Rotation|GetRotationRemainTime) 0.0)
    (Transformation|AddActorLocalRotation (Math|Rotator|MakeRotator 0.0 (* DeltaTime (/ (Variables|Rotation|GetRotationDegree) (Variables|Rotation|GetRotationTime))) 0.0) false false)
    (bind _output_get (Variables|Rotation|SetRotationRemainTime (- (Variables|Rotation|GetRotationRemainTime) DeltaTime)))
    (if (< _output_get 0.0)
      (switch Utilities|FlowControl|Switch|SwitchonEnum_PSTargetState (Variables|Components|GetTargetState)
        (:NewEnumerator3
          (Variables|Components|SetTargetState "NewEnumerator1"))
        (:NewEnumerator4
          (Variables|Components|SetTargetState "NewEnumerator2"))))))